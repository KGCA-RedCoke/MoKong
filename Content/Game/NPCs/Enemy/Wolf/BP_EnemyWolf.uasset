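; BP_EnemyWolf is a wolf enemy NPC Blueprint that adds death handling and stub perception responses to its parent class.
; On BeginPlay it binds to the ability character die event, which plays a death montage on the mesh and destroys the actor when the montage blends out.
; Seeing the player only prints a debug "Found" message with the target, and the hearing event is empty.
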(event Custom|CustomEvent
  (Animation|Montage|PlayMontage (Variables|Character|GetMesh) "/Game/Game/NPCs/Enemy/Wolf/Ability/MTG_WS_Die_Light.MTG_WS_Die_Light"
    (:OnBlendOut
      (Actor|DestroyActor))))

(event EventBeginPlay
  (|CallParentFunction)
  (EventDispatchers|BindEventtoOnAbilityCharacterDie (delegate Custom|CustomEvent)))

(event Collision|EventActorBeginOverlap
  (params (OtherActor :type Actor%20Object%20Reference))
  (|CallParentFunction OtherActor) ; 지금 이 노드는 비활성 상태입니다. \n핀을 끌어서 다른 노드를 연결하면 활성화됩니다.
)

(event EventTick
  (params (DeltaSeconds :type Float%20%28single-precision%29))
  (|CallParentFunction DeltaSeconds) ; 지금 이 노드는 비활성 상태입니다. \n핀을 끌어서 다른 노드를 연결하면 활성화됩니다.
)

(event EventOnHeardSomething
  (params (Location :type Vector%20%28by%20ref%29 :default "0, 0, 0")))

(event EventOnPlayerSeen
  (params (Target :type Actor%20Object%20Reference))
  (Development|PrintText (Utilities|Text|FormatText "Found:  {0} " Target)))

(fn ConstructionScript
  (|CallParentFunction))