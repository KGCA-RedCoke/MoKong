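; HuStone enemy character, an AI-driven melee and projectile attacker that targets the player through its Blackboard.
; Toggleable trace components on weapon, hands, foot and AOE apply the gameplay effect spec built in PreAttack.
; Gameplay tags select axe projectiles to spawn, and strong hit reactions add a Frozen state tag during the montage.
; Teleport is faked as an invisible high-speed flying AI move that ignores pawns, then reappears with a montage.
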(event Custom|TeleportEnd
  (bind _charactermovement (Variables|Character|GetCharacterMovement))
  (Components|Movement|StopMovementImmediately _charactermovement)
  (Pawn|Components|CharacterMovement|SetMovementMode _charactermovement "MOVE_Flying" 0)
  (Variables|/Script/Engine.CharacterMovementComponent|SetMaxAcceleration _charactermovement 1.5e+03)
  (Utilities|FlowControl|Delay 0.2)
  (Animation|PlayAnimMontage "/Game/Game/NPCs/Enemy/HuStone/Anim/Montages/JustMW.JustMW" 1.0 "None")
  (Rendering|SetVisibility (Variables|Character|GetMesh) true true)
  (Collision|SetCollisionResponsetoChannel (Variables|Default|GetCapsuleComponent) "ECC_Pawn" "ECR_Block")
  (Default|CallOnTeleportEnd)
  (Utilities|FlowControl|Delay 0.5)
  (Variables|Default|SetIsTeleporting false))

(event Custom|Teleport
  (params (Location :type Vector) (AttackTarget :type Actor%20Object%20Reference))
  (bind _charactermovement (Variables|Character|GetCharacterMovement))
  (Variables|Default|SetIsTeleporting true)
  (Pawn|Components|CharacterMovement|SetMovementMode _charactermovement "MOVE_Flying" 0)
  (Variables|/Script/Engine.CharacterMovementComponent|SetMaxFlySpeed _charactermovement 1e+04)
  (Variables|/Script/Engine.CharacterMovementComponent|SetMaxAcceleration _charactermovement 99999.0)
  (Rendering|SetVisibility (Variables|Character|GetMesh) false true)
  (Collision|SetCollisionResponsetoChannel (Variables|Default|GetCapsuleComponent) "ECC_Pawn" "ECR_Ignore")
  (Animation|StopAnimMontage 0)
  (AI|AIMoveTo self Location 0 15.0 false
    (:OnSuccess
      (CallFunction|TeleportEnd))))

(event EventBeginPlay
  (bind _returnvalue (Game|GetPlayerCharacter 0))
  (bind _self self)
  (bind _returnvalue_2 (AI|GetAIController _self))
  (bind _returnvalue_3 (AI|GetBlackboard _returnvalue_2))
  (|CallParentFunction)
  (Variables|Default|SetTargetActor _returnvalue)
  (AI|Components|Blackboard|SetValueasObject _returnvalue_3 (Variables|Default|GetKey%20Name) _returnvalue)
  (AI|Components|Blackboard|SetValueasObject _returnvalue_3 (Utilities|Name|MakeLiteralName "OwnerASC") (Class|MKAbilityCharacter|GetMKAbilitySystemComponent)))

(event EventTrySectionAttack
  (params (SectionName :type Name :default "None"))
  (Variables|Default|SetSectionToPlay SectionName))

(event EventAttack
  (params (AbilityClass :type MK%20Gameplay%20Ability%20Class%20Reference) (AttackType :type Byte :default 0))
  (|CallParentFunction AbilityClass AttackType))

(event EventPreAttack
  (params (Effect :type Gameplay%20Effect%20Class%20Reference) (Level :type Float%20%28single-precision%29))
  (Variables|Default|SetDamageEffect (GameplayEffects|MakeOutgoingSpec :self (Variables|Default|GetAbilitySystemComponent) :GameplayEffectClass Effect :Level (Math|Conversions|ToFloat(Integer) (Math|Float|Truncate Level)))))

(event OnItemAdded(Hand_L_AttackTrace)
  (params (LastItem :type Hit%20Result%20Structure))
  (Utilities|ApplyEffecttoTarget LastItem))

(event OnItemAdded(PrimaryAttackTrace)
  (params (LastItem :type Hit%20Result%20Structure))
  (Utilities|ApplyEffecttoTarget LastItem))

(event OnItemAdded(AOE_AttackTrace)
  (params (LastItem :type Hit%20Result%20Structure))
  (Utilities|ApplyEffecttoTarget LastItem))

(event OnItemAdded(Hand_R_AttackTrace)
  (params (LastItem :type Hit%20Result%20Structure))
  (Utilities|ApplyEffecttoTarget LastItem))

(event OnItemAdded(Foot_R_AttackTrace)
  (params (LastItem :type Hit%20Result%20Structure))
  (Utilities|ApplyEffecttoTarget LastItem))

(event Custom|EnableTrace
  (params (bEnable :type Boolean) (Type :type E_HuStone_TraceType%20Enum :default "NewEnumerator0"))
  (Class|DidItHitActorComponent|ToggleTraceCheck (Utilities|Select :Index Type :NewEnumerator0 (Variables|Default|GetPrimaryAttackTrace) :NewEnumerator1 (Variables|Default|GetHand_L_AttackTrace) :NewEnumerator2 (Variables|Default|GetHand_R_AttackTrace) :NewEnumerator3 (Variables|Default|GetFoot_R_AttackTrace) :NewEnumerator4 (Variables|Default|GetAOE_AttackTrace)) bEnable))

(event EventLaunchAttack
  (params (LaunchType :type Gameplay%20Tag%20Structure))
  (CallFunction|SPawnPro LaunchType))

(event EventPlayHitReact
  (params (ImpactLocation :type Vector%20%28by%20ref%29 :default "0, 0, 0") (Damage :type Float%20%28single-precision%29) (AdditionalTags :type Gameplay%20Tag%20Container%20Structure%20%28by%20ref%29))
  (bind _returnvalue (GameplayTags|MakeGameplayTagContainerfromTag "(TagName=\"State.AI.Frozen\")"))
  (if (GameplayTags|HasTag AdditionalTags "(TagName=\"Effect.HitLevel.Strong\")" true)
    (Animation|Montage|PlayMontage (Variables|Character|GetMesh) "/Game/Game/NPCs/Enemy/HuStone/Anim/Montages/MTG_HS_Hit.MTG_HS_Hit"
      (:then
        (Ability|GameplayEffect|AddLooseGameplayTags self _returnvalue))
      (:OnCompleted
        (Ability|GameplayEffect|RemoveLooseGameplayTags self _returnvalue :!label _label))
      (:OnBlendOut
        (goto _label))
      (:OnInterrupted
        (goto _label)))))

(fn ConstructionScript
  (|CallParentFunction)
  (Class|DidItHitActorComponent|SetupVariables (Variables|Default|GetPrimaryAttackTrace) (Variables|Character|GetMesh))
  (Class|DidItHitActorComponent|SetupVariables (Variables|Default|GetHand_L_AttackTrace) (Variables|Character|GetMesh))
  (Class|DidItHitActorComponent|SetupVariables (Variables|Default|GetHand_R_AttackTrace) (Variables|Character|GetMesh))
  (Class|DidItHitActorComponent|SetupVariables (Variables|Default|GetFoot_R_AttackTrace) (Variables|Character|GetMesh))
  (Class|DidItHitActorComponent|SetupVariables (Variables|Default|GetAOE_AttackTrace) (Variables|Character|GetMesh)))

(fn GetTargetActor
  (return (Variables|Default|GetTargetActor)))

(fn CollisionCheck
  (params (Start :type Vector) (End :type Vector) (Radius :type Float%20%28double-precision%29) (EffectLevel :type Float%20%28double-precision%29))
  (bind (_outhit _returnvalue) (Collision|SphereTraceForObjects Start End Radius (Utilities|Array|MakeArray "ObjectTypeQuery8") false 0 "ForDuration"))
  (if _returnvalue
    (bind _asmkplayer (Utilities|Casting|CastToMKPlayer (.HitActor (Collision|BreakHitResult _outhit))))
    (GameplayEffects|ApplyGameplayEffectSpecToSelf (Variables|/Script/AbilitySystem.MKAbilityCharacter|GetAbilitySystemComponent _asmkplayer) (GameplayEffects|MakeOutgoingSpec :self (Variables|Default|GetAbilitySystemComponent) :GameplayEffectClass "/Game/Game/Player/AbilitySystem/Effect/Damage/GAS_GE_StaffDamage_Light.GAS_GE_StaffDamage_Light_C" :Level EffectLevel))))

(fn SPawnPro
  (params (Tag :type Gameplay%20Tag%20Structure))
  (bind _self self)
  (|SwitchGameplayTag Tag
    (:Event.Launch.Tornado
      (LocalVariables|SetLocal_SocketName "None")
      (LocalVariables|SetLocalSpawnActor "/Game/Game/NPCs/Enemy/HuStone/Projectiles/BP_Projectile_AxeTornado.BP_Projectile_AxeTornado_C"))
    (:Event.Launch.AirBlade
      (LocalVariables|SetLocal_SocketName "TraceStart")
      (LocalVariables|SetLocalSpawnActor "/Game/Game/NPCs/Enemy/HuStone/Projectiles/BP_Projectile_SpinningAxe.BP_Projectile_SpinningAxe_C")))
  (Game|SpawnActorfromClass (LocalVariables|GetLocalSpawnActor) (Math|Transform|MakeTransform (Transformation|GetSocketLocation (Variables|Character|GetMesh) (LocalVariables|GetLocal_SocketName)) "0, 0, 0" "1.000000,1.000000,1.000000") "Undefined" "MultiplyWithRoot" _self _self))

(fn GetPatrolRoute
  (return 0))