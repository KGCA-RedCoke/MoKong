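; Background music manager actor that switches tracks on a single audio component with fades.
; BeginPlay attempts a singleton through an Instance variable, destroying the actor if it is already set.
; PlayBGM ignores the current track, otherwise fades out any playing audio and uses function-name timers to stop it and start the new one.
; When nothing plays, it also calls StartNewBGM immediately, before CurrentBGM updates.
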(event EventBeginPlay
  (if (== (Variables|Default|GetInstance) 0)
    (Variables|Default|SetInstance self)
    (else
      (Actor|DestroyActor))))

(event Collision|EventActorBeginOverlap
  (params (OtherActor :type Actor%20Object%20Reference)))

(event EventTick
  (params (DeltaSeconds :type Float%20%28single-precision%29)))

(fn ConstructionScript)

(fn PlayBGM
  (params (NewBGM :type Sound%20Base%20Object%20Reference))
  (bind _fadeouttime (Variables|Default|GetFadeOutTime))
  (LocalVariables|SetNewLocalBGM NewBGM)
  (if (== NewBGM (Variables|Default|GetCurrentBGM))
    (return)
    (else
      (if (Audio|Components|Audio|IsPlaying (Variables|Default|GetAudio))
        (Audio|Components|Audio|FadeOut (Variables|Default|GetAudio) _fadeouttime 0.0 "Linear" :!class /Script/Engine.AudioComponent)
        (Utilities|Time|SetTimerbyFunctionName 0 "StopCurrentBGM" _fadeouttime)
        (else
          (CallFunction|StartNewBGM)))
      (Variables|Default|SetCurrentBGM (LocalVariables|GetNewLocalBGM))
      (Utilities|Time|SetTimerbyFunctionName 0 "StartNewBGM" _fadeouttime)
      (return))))

(fn StopCurrentBGM
  (Audio|Components|Audio|Stop (Variables|Default|GetAudio))
  (return))

(fn StartNewBGM
  (bind _audio (Variables|Default|GetAudio))
  (Audio|Components|Audio|SetSound (Variables|Default|GetAudio) (Variables|Default|GetCurrentBGM))
  (Audio|Components|Audio|FadeIn _audio (Variables|Default|GetFadeInTime) 1.0 0.0 "Linear" :!class /Script/Engine.AudioComponent)
  (Audio|Components|Audio|Play _audio 0.0)
  (return))