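; BP_MKBoss is a boss enemy Blueprint that adds death presentation on top of its parent class.
; On BeginPlay it binds to the ability character's die event and plays the Dead_Forward montage when that fires.
; The construction script hides the inherited enemy HP widget.
; EnableTrace is an empty stub, and the FX-then-destroy step noted in a comment has no logic here.
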(event Custom|CustomEvent
  ;[0.01096 0.01161 0.0137] FX 재생하고 끝나면 Destroy 호출
  (Animation|PlayAnimMontage "/Game/Game/NPCs/Enemy/HuStone/Anim/Montages/Dead_Forward.Dead_Forward" 1.0 "None"))

(event EventBeginPlay
  (|CallParentFunction)
  ;[0.01096 0.01161 0.0137] FX 재생하고 끝나면 Destroy 호출
  (EventDispatchers|BindEventtoOnAbilityCharacterDie (delegate Custom|CustomEvent)))

(event Collision|EventActorBeginOverlap
  (params (OtherActor :type Actor%20Object%20Reference))
  (|CallParentFunction OtherActor) ; 지금 이 노드는 비활성 상태입니다. \n핀을 끌어서 다른 노드를 연결하면 활성화됩니다.
)

(event EventTick
  (params (DeltaSeconds :type Float%20%28single-precision%29))
  (|CallParentFunction DeltaSeconds) ; 지금 이 노드는 비활성 상태입니다. \n핀을 끌어서 다른 노드를 연결하면 활성화됩니다.
)

(event Custom|EnableTrace
  (params (bEnable :type Boolean) (Type :type E_HuStone_TraceType%20Enum :default "NewEnumerator0")))

(fn ConstructionScript
  (|CallParentFunction)
  (Rendering|SetVisibility (Variables|Default|GetEnemyHPWidgetComponent) false false))