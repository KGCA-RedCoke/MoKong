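; BP_MKEnemy is a base enemy character using the Gameplay Ability System, with an HP widget and lock-on socket.
; It serves AI queries for target, patrol, range and speed, tagging itself attacking when it sees a target.
; Attacks go through gameplay events or ability activation; hit reactions choose montage by direction and section by strength, tagging AI frozen meanwhile.
; Death unpossesses, plays a montage, drops items and destroys the actor after a delay.
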(event EventBeginPlay
  (bind _aswbp_enemy (Utilities|Casting|CastToWBP_Enemy (UserInterface|GetWidget (Variables|Default|GetEnemyHPWidgetComponent))))
  (Variables|Default|SetBarWidget _aswbp_enemy)
  (Class|AbilityBindWidgetBase|InitializeAbilitySystemWidget (Variables|Default|GetBarWidget) (Variables|Default|GetAbilitySystemComponent)))

(event Collision|EventActorBeginOverlap
  (params (OtherActor :type Actor%20Object%20Reference)))

(event EventTick
  (params (DeltaSeconds :type Float%20%28single-precision%29)))

(event EventOnDeath
  (|CallParentFunction)
  (Development|PrintText "죽었을 때를 여기서 구현하세요. 이게 뜨면 구현이 안된 것")
  (Pawn|UnPossess (AI|GetAIController self))
  (Animation|Montage|PlayMontage (Variables|Character|GetMesh) (Variables|Default|GetDeathMontage)
    (:then
      (Class|MokongEnemy|GenDeathItems)
      (Utilities|FlowControl|Delay 6.0)
      (Actor|DestroyActor))))

(event EventOnPlayerSeen
  (params (Target :type Actor%20Object%20Reference))
  (bind _returnvalue (GameplayTags|MakeLiteralGameplayTagContainer "(GameplayTags=((TagName=\"State.AI.Attacking\")))"))
  (bind _self self)
  ;[0.01096 0.01161 0.0137] 기본적으로 플레이어를 발견하면 타겟으로 지정
  (bind _output_get (Variables|Default|SetTargetActor Target))
  (Utilities|IsValid _output_get
    (:Is%20Valid
      (Ability|GameplayEffect|AddLooseGameplayTags _self _returnvalue))
    (:Is%20Not%20Valid
      (Ability|GameplayEffect|RemoveLooseGameplayTags _self _returnvalue))))

(event EventAttack
  (params (AbilityClass :type MK%20Gameplay%20Ability%20Class%20Reference) (AttackType :type Byte :default 0))
  (bind _montagemap (Variables|Default|GetMontageMap))
  (bind (_value _returnvalue) (Utilities|Map|Find _montagemap AttackType))
  (if _returnvalue
    (Ability|SendGameplayEventtoActor self "(TagName=\"Event.Task.StartAttack\")" (Utilities|Struct|MakeGameplayEventData "(TagName=\"\")" 0 0 _value))))

(event EventOnHeardSomething
  (params (Location :type Vector%20%28by%20ref%29 :default "0, 0, 0"))
  ;[0.01096 0.01161 0.0137] 뭘 듣거나 시체 발견시 조사하거나
)

(event EventPlayHitReact
  (params (ImpactLocation :type Vector%20%28by%20ref%29 :default "0, 0, 0") (Damage :type Float%20%28single-precision%29) (AdditionalTags :type Gameplay%20Tag%20Container%20Structure%20%28by%20ref%29))
  (bind _returnvalue (GameplayTags|MakeGameplayTagContainerfromTag "(TagName=\"State.AI.Frozen\")"))
  (|CallParentFunction ImpactLocation Damage AdditionalTags)
  (bind (_montagetoplay _sectiontoplay) (CallFunction|HandleHitReaction ImpactLocation Damage AdditionalTags))
  (Utilities|IsValid _montagetoplay
    (:Is%20Valid
      (Animation|Montage|PlayMontage (Variables|Character|GetMesh) _montagetoplay 1.0 0.0 _sectiontoplay
        (:then
          (Ability|GameplayEffect|AddLooseGameplayTags self _returnvalue))
        (:OnBlendOut
          (Ability|GameplayEffect|RemoveLooseGameplayTags self _returnvalue :!label _label))
        (:OnInterrupted
          (goto _label))))))

(event EventTryComboAttack
  (Abilities|TryActivateAbilitybyClass (Variables|Default|GetAbilitySystemComponent) "/Game/Game/NPCs/Enemy/Base/Ability/GAS_GA_EnemyAttackBase.GAS_GA_EnemyAttackBase_C" true))

(fn ConstructionScript
  (Transformation|AttachComponentToComponent (Variables|Default|GetLockOnWidgetComponent) (Variables|Character|GetMesh) "CAMERA_LOCK" "SnapToTarget" "SnapToTarget" "SnapToTarget" false))

(fn SetMovementSpeed
  (params (NewSpeed :type EAIMovementSpeed%20Enum :default "Patrol"))
  (bind _output_get (Variables|/Script/Engine.CharacterMovementComponent|SetMaxWalkSpeed (Variables|Character|GetCharacterMovement) (Utilities|Select :Index NewSpeed :Patrol 1e+02 :Chase 5e+02 :Attack 1.5e+02 :ETC1 0.0 :ETC2 0.0 :ETC3 0.0 :ETC4 0.0 :ETC5 0.0)))
  (return _output_get))

(fn GetIdealRange
  (return 3e+02 3e+02))

(fn GetTargetActor
  (return (Variables|Default|GetTargetActor)))

(fn HandleHitReaction
  (params (ImpactPoint :type Vector) (Damage :type Float%20%28double-precision%29) (Tags :type Gameplay%20Tag%20Container%20Structure))
  (bind _hitreactmontages_front (Variables|Default|GetHitReactMontages_Front))
  (if (GameplayTags|HasMatchingGameplayTag (Variables|Default|GetAbilitySystemComponent) "(TagName=\"Immunity.HitReact\")")
    (return 0 "None")
    (else
      (LocalVariables|SetL_Strong? (GameplayTags|HasTag Tags "(TagName=\"Effect.HitLevel.Strong\")" true))
      (LocalVariables|SetL_Frozen? (GameplayTags|HasTag Tags "(TagName=\"Effect.HitLevel.Frozen\")" true))
      ;[0.01096 0.01161 0.0137] 방향에 따라 몽타주 결정
      (bind _returnvalue (Class|MokongBlueprintFunctionLibrary|GetHitDirection self ImpactPoint))
      (return (Utilities|Select :Index _returnvalue :None _hitreactmontages_front :Forward _hitreactmontages_front :Left (Variables|Default|GetHitReactMontages_Left) :Right (Variables|Default|GetHitReactMontages_Right) :Backward (Variables|Default|GetHitReactMontages_Back)) (Utilities|String|StringToName (Utilities|String|Append (LocalVariables|GetL_Section) (Utilities|String|SelectString "3" (Utilities|String|SelectString "2" "1" (LocalVariables|GetL_Strong?)) (LocalVariables|GetL_Frozen?))))))))

(fn OnHitPlayer
  (params (LastItem :type Hit%20Result%20Structure))
  ;[0.01096 0.01161 0.0137] 부모는 항상 호출
  ; (아예 독립적인 로직을 작성하려면 부모 생략)
  (|CallParentFunction LastItem)
  (Development|PrintText "플레이어 때렸을 때 추가 구현할게 있으면 여기서하세요 
( MKEnemy -> OnHitPlayer)"))

(fn GetPatrolRoute
  (return (Variables|Enemy|AI|GetPatrol%20Route)))