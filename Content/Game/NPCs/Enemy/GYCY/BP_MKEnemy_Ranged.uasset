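; Ranged bow enemy Blueprint that targets the first player character.
; On BeginPlay it stores the player as its target and passes the player and its own ability system component to the AI blackboard.
; Attack draws the bow through ACBowMechanics, then after a short delay fires with the target's location and the MontageMap entry.
; Strong hits play a reaction montage, holding the State.AI.Frozen tag until it ends.
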(event EventBeginPlay
  (bind _returnvalue (Game|GetPlayerCharacter 0))
  (bind _self self)
  (bind _returnvalue_2 (AI|GetAIController _self))
  (bind _returnvalue_3 (AI|GetBlackboard _returnvalue_2))
  (|CallParentFunction)
  (Variables|Default|SetTargetActor _returnvalue)
  (AI|Components|Blackboard|SetValueasObject _returnvalue_3 (Variables|Default|GetKey%20Name) _returnvalue)
  (AI|Components|Blackboard|SetValueasObject _returnvalue_3 (Utilities|Name|MakeLiteralName "OwnerASC") (Class|MKAbilityCharacter|GetMKAbilitySystemComponent)))

(event EventAttack
  (params (AbilityClass :type MK%20Gameplay%20Ability%20Class%20Reference) (AttackType :type Byte :default 0))
  (bind _montagemap (Variables|Default|GetMontageMap))
  (bind (_value _returnvalue) (Utilities|Map|Find _montagemap AttackType))
  (if _returnvalue
    (Default|DrawBegin (Variables|Default|GetAC_BowMechanics))
    (Utilities|FlowControl|Delay 0.2)
    (Default|FireArrowBegin (Variables|Default|GetAC_BowMechanics) (Transformation|GetActorLocation (Variables|Default|GetTargetActor)) _value)))

(event EventTick
  (params (DeltaSeconds :type Float%20%28single-precision%29))
  (|CallParentFunction DeltaSeconds) ; 지금 이 노드는 비활성 상태입니다. \n핀을 끌어서 다른 노드를 연결하면 활성화됩니다.
)

(event Collision|EventActorBeginOverlap
  (params (OtherActor :type Actor%20Object%20Reference))
  (|CallParentFunction OtherActor) ; 지금 이 노드는 비활성 상태입니다. \n핀을 끌어서 다른 노드를 연결하면 활성화됩니다.
)

(event EventPlayHitReact
  (params (ImpactLocation :type Vector%20%28by%20ref%29 :default "0, 0, 0") (Damage :type Float%20%28single-precision%29) (AdditionalTags :type Gameplay%20Tag%20Container%20Structure%20%28by%20ref%29))
  (bind _returnvalue (GameplayTags|MakeGameplayTagContainerfromTag "(TagName=\"State.AI.Frozen\")"))
  (if (GameplayTags|HasTag AdditionalTags "(TagName=\"Effect.HitLevel.Strong\")" true)
    (Animation|Montage|PlayMontage (Variables|Character|GetMesh) "/Game/Game/NPCs/Enemy/GYCY/Range/MTG_GYCY_Ranged_Hit.MTG_GYCY_Ranged_Hit"
      (:then
        (Ability|GameplayEffect|AddLooseGameplayTags self _returnvalue))
      (:OnCompleted
        (Ability|GameplayEffect|RemoveLooseGameplayTags self _returnvalue :!label _label))
      (:OnBlendOut
        (goto _label))
      (:OnInterrupted
        (goto _label)))))

(fn ConstructionScript
  (|CallParentFunction))