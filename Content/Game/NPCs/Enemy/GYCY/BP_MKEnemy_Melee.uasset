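; Melee enemy NPC Blueprint that targets the player and attacks with a traced weapon.
; On BeginPlay it stores the player character as its target and writes its MK Ability System Component to the AI controller's blackboard.
; It also binds the primary attack trace to its weapon mesh and itself.
; GetIdealRange supplies fixed attack and detection distances; Tick and overlap events are unused.
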(event EventBeginPlay
  (|CallParentFunction)
  (Variables|Default|SetTargetActor (Game|GetPlayerCharacter 0))
  (AI|Components|Blackboard|SetValueasObject (AI|GetBlackboard (AI|GetAIController self)) (Utilities|Name|MakeLiteralName "OwnerASC") (Class|MKAbilityCharacter|GetMKAbilitySystemComponent))
  (Class|DidItHitActorComponent|SetupVariables (Variables|Default|GetPrimaryAttackTrace) (Variables|Default|GetWeaponMesh) self))

(event Collision|EventActorBeginOverlap
  (params (OtherActor :type Actor%20Object%20Reference))
  (|CallParentFunction OtherActor) ; 지금 이 노드는 비활성 상태입니다. \n핀을 끌어서 다른 노드를 연결하면 활성화됩니다.
)

(event EventTick
  (params (DeltaSeconds :type Float%20%28single-precision%29))
  (|CallParentFunction DeltaSeconds) ; 지금 이 노드는 비활성 상태입니다. \n핀을 끌어서 다른 노드를 연결하면 활성화됩니다.
)

(fn ConstructionScript
  (|CallParentFunction))

(fn GetTargetActor
  (return 0))

(fn GetIdealRange
  (return 4.5e+02 1e+03))