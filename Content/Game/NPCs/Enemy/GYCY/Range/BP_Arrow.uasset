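; Arrow projectile, likely for a ranged enemy, that damages or affects an MKPlayer through a supplied gameplay effect spec.
; Fire adds projectile movement at runtime, scaling speed and gravity by Strength, and starts whoosh, trail and spin.
; Any non-instigator overlap halts it, but only player hits apply the spec, attach near the closest bone, play impact effects and broadcast the impact.
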(event OnComponentBeginOverlap(CollisionBox)
  (params (OverlappedComponent :type Primitive%20Component%20Object%20Reference) (OtherActor :type Actor%20Object%20Reference) (OtherComp :type Primitive%20Component%20Object%20Reference) (OtherBodyIndex :type Integer) (bFromSweep :type Boolean) (SweepResult :type Hit%20Result%20Structure%20%28by%20ref%29))
  (bind (_bblockinghit _binitialoverlap _time _distance _location _impactpoint _normal _impactnormal _physmat _hitactor _hitcomponent) (Collision|BreakHitResult SweepResult))
  (bind _returnvalue (Actor|GetComponentbyClass _hitactor "/Script/Engine.SkeletalMeshComponent"))
  (if (!= OtherActor (Game|GetInstigator))
    (bind _projectilemovementcomponent (Variables|Default|GetProjectileMovementComponent)
      (:then
        (Components|DestroyComponent _projectilemovementcomponent))
      (:else
        _))
    (Collision|SetCollisionEnabled (Variables|Default|GetCollisionBox) "NoCollision")
    (bind _asmkplayer (Utilities|Casting|CastToMKPlayer _hitactor))
    (GameplayEffects|ApplyGameplayEffectSpecToSelf (Variables|/Script/AbilitySystem.MKAbilityCharacter|GetAbilitySystemComponent _asmkplayer) (Variables|Default|GetSpec%20Handle))
    (Audio|Components|Audio|Stop (Variables|Default|GetSpinArrowTimeline))
    (Utilities|IsValid _returnvalue
      (:Is%20Valid
        (Transformation|AttachComponentToComponent _returnvalue (Class|SkinnedMeshComponent|GetParentBone _returnvalue (.ReturnValue (Class|SkinnedMeshComponent|FindClosestBoneK2 _returnvalue _location 0.0))) "SnapToTarget" "KeepWorld" "KeepWorld" true))
      (:Is%20Not%20Valid
        (Transformation|AttachComponentToComponent _hitcomponent "None" "KeepWorld" "KeepWorld" "KeepWorld" true)))
    (Audio|PlaySoundatLocation (Variables|Default|GetImpactSound) (Transformation|GetActorLocation) "0, 0, 0" 1.0 1.0 0.0 0 0 0 0)
    (Effects|SpawnEmitteratLocation (Variables|Default|GetImpactEffect) _location)
    (if (Physics|IsSimulatingPhysics _hitcomponent "None")
      (Physics|AddImpulse _hitcomponent (Variables|Default|GetVelocity) "None" true))
    (Default|CallOnArrowImpact (Variables|Default|GetStrength) _hitactor SweepResult)
    (Utilities|FlowControl|Delay 1.0)
    (bind _traileffectref (Variables|Default|GetTrailEffectRef)
      (:then
        (Components|DestroyComponent _traileffectref))
      (:else))))

(event Custom|Fire
  (params (Direction :type Vector) (Strength :type Float%20%28double-precision%29))
  (bind _returnvalue (AddComponent|AddProjectileMovementComponent))
  (Variables|Default|SetProjectileMovementComponent _returnvalue)
  (bind _output_get (Variables|/Script/Engine.MovementComponent|SetVelocity _returnvalue (* Direction (Math|Float|Lerp (Variables|Default|GetMinSpeed) (Variables|Default|GetMaxSpeed) Strength))))
  (Variables|Default|SetVelocity _output_get)
  (Variables|/Script/Engine.ProjectileMovementComponent|SetProjectileGravityScale _returnvalue (Math|Float|Lerp (Variables|Default|GetMaxGravity) (Variables|Default|GetMinGravity) Strength))
  (Audio|PlaySoundatLocation (Variables|Default|GetWhooshSound) (Transformation|GetActorLocation) "0, 0, 0" 1.0 1.0 0.0 0 0 0 0)
  (bind _returnvalue_2 (Niagara|SpawnSystemAttached (Variables|Default|GetTrailEffect) (Variables|Default|GetTrailEffectLocation) "None" "0, 0, 0" "0, 0, 0" "KeepRelativeOffset" false))
  (Variables|Default|SetTrailEffectRef _returnvalue_2)
  (Collision|SetCollisionEnabled (Variables|Default|GetCollisionBox) "QueryAndPhysics")
  (Actor|SetLifeSpan 5.0)
  (CallFunction|SpinStart)
  (Variables|Default|SetStrength Strength))

(event Custom|SpinStart
  (bind _xrotation (Timeline|SpinArrowTimeline PlayFromStart)
    (:Update
      (Transformation|SetRelativeRotation (Variables|Default|GetArrowMesh) (Math|Rotator|MakeRotator _xrotation 0.0 0.0) false false))))

(event EventBeginPlay
  (Collision|SetCollisionEnabled (Variables|Default|GetCollisionBox) "NoCollision"))

(fn ConstructionScript)

(fn NewFunction
  (params (Object :type Object%20Object%20Reference)))