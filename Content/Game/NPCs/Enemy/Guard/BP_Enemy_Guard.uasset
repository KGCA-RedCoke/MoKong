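; BP_Enemy_Guard is a Guard enemy NPC Blueprint whose own logic handles the death sequence.
; On BeginPlay it binds to the ability character's die event and to the DeathFX system-finished event.
; Death plays a demon death montage and hides the lock-on widget.
; A montage notify activates DeathFX, and the actor is destroyed when that effect finishes.
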(event Custom|PlayFX
  (params (PSystem :type Niagara%20Component%20Object%20Reference))
  (Actor|DestroyActor))

(event Custom|OnAbilityCharacterDie_이벤트
  (Animation|Montage|PlayMontage (Variables|Character|GetMesh) "/Game/Characters/DemonGuard/Animations/MTG_Demon_Death.MTG_Demon_Death"
    (:then
      (Rendering|SetVisibility (Variables|Default|GetLockOnWidgetComponent) false false))
    (:OnNotifyBegin
      (Components|Activation|SetActive (Variables|Default|GetDeathFX) true false))))

(event EventBeginPlay
  (EventDispatchers|BindEventtoOnSystemFinished (Variables|Default|GetDeathFX) (delegate Custom|PlayFX))
  (EventDispatchers|AssignOnAbilityCharacterDie (delegate Custom|OnAbilityCharacterDie_이벤트)))

(fn ConstructionScript)