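; Guangzhi enemy NPC Blueprint that attacks through the Gameplay Ability System and targets the first player.
; BeginPlay writes the player and its own ability component to the AI Blackboard.
; PreAttack builds a damage effect spec, which toggleable attack traces apply to hit actors with an ability component.
; Hit reactions play a montage and add a Frozen tag, whose removal is unwired; a separate sphere-trace check applies light staff damage.
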(event Custom|BaseAttack_1
  (params (AttackType :type E_HuStone_Attacks%20Enum :default "NewEnumerator0") (AbilityToActivate :type MK%20Gameplay%20Ability%20Class%20Reference))
  (Variables|Default|SetAttackType AttackType)
  (Abilities|TryActivateAbilitybyClass (Class|MKAbilityCharacter|GetMKAbilitySystemComponent) (select (Utilities|IsValidClass AbilityToActivate) 0 0) true))

(event EventBeginPlay
  (bind _returnvalue (Game|GetPlayerCharacter 0))
  (bind _self self)
  (bind _returnvalue_2 (AI|GetAIController _self))
  (bind _returnvalue_3 (AI|GetBlackboard _returnvalue_2))
  (|CallParentFunction)
  (Variables|Default|SetTargetActor _returnvalue)
  (AI|Components|Blackboard|SetValueasObject _returnvalue_3 (Variables|Default|GetKey%20Name) _returnvalue)
  (AI|Components|Blackboard|SetValueasObject _returnvalue_3 (Utilities|Name|MakeLiteralName "OwnerASC") (Class|MKAbilityCharacter|GetMKAbilitySystemComponent))
  (Class|DidItHitActorComponent|SetupVariables (Variables|Default|GetPrimaryAttackTrace) (Variables|Default|GetSK_Weapon)))

(event EventTrySectionAttack
  (params (SectionName :type Name :default "None"))
  (Variables|Default|SetSectionToPlay SectionName))

(event EventPreAttack
  (params (Effect :type Gameplay%20Effect%20Class%20Reference) (Level :type Float%20%28single-precision%29))
  (Variables|Default|SetDamageEffect (GameplayEffects|MakeOutgoingSpec :self (Variables|Default|GetAbilitySystemComponent) :GameplayEffectClass Effect :Level (Math|Conversions|ToFloat(Integer) (Math|Float|Truncate Level)))))

(event EventPlayHitReact
  (params (ImpactLocation :type Vector%20%28by%20ref%29 :default "0, 0, 0") (Damage :type Float%20%28single-precision%29) (AdditionalTags :type Gameplay%20Tag%20Container%20Structure%20%28by%20ref%29))
  (Animation|Montage|PlayMontage (Variables|Character|GetMesh) 0 1.0 0.0 "BH1_L"
    (:then
      (Ability|GameplayEffect|AddLooseGameplayTags self (GameplayTags|MakeGameplayTagContainerfromTag "(TagName=\"State.AI.Frozen\")")))))

(event EventAttack
  (params (AbilityClass :type MK%20Gameplay%20Ability%20Class%20Reference) (AttackType :type Byte :default 0))
  (|CallParentFunction AbilityClass AttackType))

(event OnItemAdded(CHBAttackTrace)
  (params (LastItem :type Hit%20Result%20Structure))
  (Utilities|ApplyEffecttoTarget LastItem))

(event OnItemAdded(PrimaryAttackTrace)
  (params (LastItem :type Hit%20Result%20Structure))
  (Utilities|ApplyEffecttoTarget LastItem))

(event OnItemAdded(SwordAttackTrace)
  (params (LastItem :type Hit%20Result%20Structure))
  (Utilities|ApplyEffecttoTarget LastItem))

(event Custom|EnableTrace
  (params (bEnable :type Boolean) (Type :type E_HuStone_TraceType%20Enum :default "NewEnumerator0"))
  (Class|DidItHitActorComponent|ToggleTraceCheck (Utilities|Select :Index Type :NewEnumerator0 (Variables|Default|GetSwordAttackTrace) :NewEnumerator1 0 :NewEnumerator2 0 :NewEnumerator3 (Variables|Default|GetCHBAttackTrace) :NewEnumerator4 0) bEnable))

(fn ConstructionScript
  (|CallParentFunction)
  (Class|DidItHitActorComponent|SetupVariables (Variables|Default|GetPrimaryAttackTrace) (Variables|Character|GetMesh))
  (Class|DidItHitActorComponent|SetupVariables (Variables|Default|GetSwordAttackTrace) (Variables|Character|GetMesh))
  (Class|DidItHitActorComponent|SetupVariables (Variables|Default|GetCHBAttackTrace) (Variables|Character|GetMesh)))

(fn GetTargetActor
  (return (Variables|Default|GetTargetActor)))

(fn CollisionCheck
  (params (Start :type Vector) (End :type Vector) (Radius :type Float%20%28double-precision%29) (EffectLevel :type Float%20%28double-precision%29))
  (bind (_outhit _returnvalue) (Collision|SphereTraceForObjects Start End Radius (Utilities|Array|MakeArray "ObjectTypeQuery8") false 0 "ForDuration"))
  (if _returnvalue
    (bind _asmkplayer (Utilities|Casting|CastToMKPlayer (.HitActor (Collision|BreakHitResult _outhit))))
    (GameplayEffects|ApplyGameplayEffectSpecToSelf (Variables|/Script/AbilitySystem.MKAbilityCharacter|GetAbilitySystemComponent _asmkplayer) (GameplayEffects|MakeOutgoingSpec :self (Variables|Default|GetAbilitySystemComponent) :GameplayEffectClass "/Game/Game/Player/AbilitySystem/Effect/Damage/GAS_GE_StaffDamage_Light.GAS_GE_StaffDamage_Light_C" :Level EffectLevel))))

(fn 새함수)