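; AI controller for crowd NPCs that reacts to sight and hearing perception.
; Perception updates are sorted by sense class: sight calls the sight handler and sets the blackboard target, using an empty value when sight is lost.
; Successfully sensed sounds pass their location to the hearing handler.
; Unpossessing clears the forgotten-actors timer, and the forgot-actor handler is left empty.
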(event OnTargetPerceptionUpdated(PerceptionComponent)
  (params (Actor :type Actor%20Object%20Reference) (Stimulus :type AI%20Stimulus%20Structure))
  (bind (_stimuluslocation _bsuccessfullysensed) (Utilities|Struct|BreakAIStimulus Stimulus))
  (bind _returnvalue (select _bsuccessfullysensed Actor 0))
  (Utilities|ClssifyStimulus Stimulus
    (:Sight
      (Class|CrowdEnemyAIController|HandleSenseSight _returnvalue)
      (AI|Components|Blackboard|SetValueasObject (AI|GetBlackboard 0) (Variables|Default|GetKey_Target) _returnvalue))
    (:Sound
      (if _bsuccessfullysensed
        (Class|CrowdEnemyAIController|HandleSenseHearing _stimuluslocation)))))

(event EventPossess
  (params (PossessedPawn :type Pawn%20Object%20Reference))
  (|CallParentFunction PossessedPawn))

(event EventUnPossess
  (params (UnpossessedPawn :type Pawn%20Object%20Reference))
  (|CallParentFunction UnpossessedPawn)
  (Utilities|Time|ClearandInvalidateTimerbyHandle (Variables|Default|GetCheckForgottenActorsTimer)))

(fn ConstructionScript)

(fn HandleForgotActor
  (params (Actor :type Actor%20Object%20Reference)))