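; Player character Blueprint that sets up animation layers, camera lock-on feedback and a weapon-sheathing key.
; BeginPlay links the base anim layer and binds the camera's target-change delegate, which shows the lock-on widget or hides it and clears the target on loss.
; Blueprint locomotion and parkour components are handed to C++ variables per instance rather than on the CDO.
; A sphere-trace guard-targeting chain remains unconnected.
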(event Custom|OnTargetChangeDelegate_이벤트
  (params (NewTarget :type Actor%20Object%20Reference) (ChangeTargetReason :type EATPCChangeTargetReason%20Enum :default "SetNew"))
  (bind _target (Variables|Default|GetTarget)
    (:then
      (switch Utilities|FlowControl|Switch|SwitchonEATPCChangeTargetReason ChangeTargetReason
        (:SetNew
          (Class|MokongEnemy|ShowLockonWidget _target true))
        (:LostByExitCameraMode
          (Class|MokongEnemy|ShowLockonWidget _target false :!label _label)
          (Variables|Default|SetTarget 0))
        (:LostByDistance
          (goto _label))
        (:LostByVisible
          (goto _label))
        (:LostByPlayerInput
          (goto _label))))
    (:else)))

(event EventBeginPlay
  (Components|SkeletalMesh|AnimationBlueprintLinking|LinkAnimClassLayers (Variables|Character|GetMesh) "/Game/Game/Player/MovementSystem/Animation/Layer/ABP_UE5_Layer_Base.ABP_UE5_Layer_Base_C")
  (EventDispatchers|AssignOnTargetChangeDelegate (Class|ATPCCameraComponent|GetCameraLockonTargetObject (Variables|Default|GetPlayerCam)) (delegate Custom|OnTargetChangeDelegate_이벤트)))

(event Input|KeyboardEvents|X
  (params (Key :type Key%20Structure :default "None"))
  (:Pressed
    (Class|WeaponBase|SheathWeapon (Variables|/Script/AbilitySystem.CombatSystem|GetCurrentWeapon (Variables|Default|GetCombatComponent)))))

(fn ConstructionScript
  (|BP->C++))