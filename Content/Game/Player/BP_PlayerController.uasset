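; BP_PlayerController is the player controller that adds the Enhanced Input mapping context and creates the player's UI.
; On BeginPlay it creates the HUD widget, retrying each tick until it initializes with the controlled pawn's Ability System Component, then adds it to the viewport.
; P toggles a lazily created ability UI and sets the cursor, taking the hide-side value from SetGamePaused(false)'s return.
; The SetGamePaused(true) nodes are unconnected.
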(event EventBeginPlay
  (Input|AddMappingContext (PlayerController|LocalPlayerSubsystems|GetEnhancedInputLocalPlayerSubsystem self) "/Game/Game/Data/Input/InputMappingContext.InputMappingContext" 0 "(bIgnoreAllPressedKeysUntilRelease=True,bForceImmediately=False,bNotifyUserSettings=False)")
  (bind _returnvalue (UserInterface|CreateWidget "/Game/Game/UI/Player/HUD/WBP_PlayerHUDWidget.WBP_PlayerHUDWidget_C" self))
  (bind _output_get (Variables|Default|SetPlayerAttributeWidget _returnvalue))
  (Utilities|IsValid _output_get
    (:Is%20Valid
      (bind _returnvalue_2 (Class|PlayerHUDWidget|InitializeAbilitySystemWidget _output_get (Ability|GetAbilitySystemComponent (Pawn|GetControlledPawn)) :!label _label))
      (if _returnvalue_2
        (UserInterface|Viewport|AddtoViewport (Variables|Default|GetPlayerAttributeWidget) 0)
        (else
          (Utilities|FlowControl|DelayUntilNextTick)
          (goto _label))))))

(event EventTick
  (params (DeltaSeconds :type Float%20%28single-precision%29)))

(event Input|KeyboardEvents|P
  (params (Key :type Key%20Structure :default "None"))
  (:Pressed
    (Utilities|FlowControl|FlipFlop
      (:A
        (bind _attwidget (Variables|Default|GetAttWidget)
          (:then
            (Widget|SetVisibility _attwidget "Visible")
            (Variables|Default|SetbShowMouseCursor true))
          (:else
            (bind _returnvalue (UserInterface|CreateWidget "/Game/Game/UI/HUD/AbilityUI/WBP_AbilityUI.WBP_AbilityUI_C" self))
            (Variables|Default|SetAttWidget _returnvalue)
            (UserInterface|Viewport|AddtoViewport (Variables|Default|GetAttWidget) 0)
            (Variables|Default|SetbShowMouseCursor true))))
      (:B
        (Widget|SetVisibility (Variables|Default|GetAttWidget) "Collapsed")
        (bind _returnvalue_2 (Game|SetGamePaused false))
        (Variables|Default|SetbShowMouseCursor _returnvalue_2)))))

(fn ConstructionScript)