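; Player character Blueprint for Wukong, handling lock-on, primary attack input and a test key for drinking the gourd.
; Lock-on input toggles the camera's target, acquiring a MokongEnemy through a forward sphere trace or clearing the current one.
; Primary action defers to CombatComponent, while the gourd test plays a montage and applies a GAS effect.
; A "BP -> C++" graph assigns Blueprint locomotion and parkour components to C++ references, as they are not CDO-initialized.
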(event Input|EnhancedActionEvents|EnhancedInputActionInputAction_Lockon
  (params (ActionValue :type Boolean) (ElapsedSeconds :type Float%20%28double-precision%29) (TriggeredSeconds :type Float%20%28double-precision%29) (InputAction :type Input%20Action%20Object%20Reference :default "/Game/Game/Data/Input/InputAction_Lockon.InputAction_Lockon"))
  (:Started
    (Utilities|IsValid (Class|ATPCCameraLockonTargetObject|GetTargetActor (Class|ATPCCameraComponent|GetCameraLockonTargetObject (Variables|Default|GetPlayerCameraComponent)))
      (:Is%20Valid
        (Utilities|HandleLockon 1e+03 :!label _label))
      (:Is%20Not%20Valid
        (goto _label TryLockOn)))))

(event Input|EnhancedActionEvents|EnhancedInputActionInputAction_PrimaryAction
  (params (ActionValue :type Boolean) (ElapsedSeconds :type Float%20%28double-precision%29) (TriggeredSeconds :type Float%20%28double-precision%29) (InputAction :type Input%20Action%20Object%20Reference :default "/Game/Game/Data/Input/InputAction_PrimaryAction.InputAction_PrimaryAction"))
  (:Started
    (Class|CombatSystem|CheckCommit (Variables|Default|GetCombatComponent))))

(event Input|KeyboardEvents|X
  (params (Key :type Key%20Structure :default "None"))
  ;[0.01096 0.01161 0.0137] Test
  (:Pressed
    (Animation|PlayAnimMontage "/Game/Game/Player/Animation/Montages/MTG_Gourd_1.MTG_Gourd_1" 1.0 "None")
    (GameplayEffects|ApplyGameplayEffectToSelf :self (Variables|Default|GetAbilitySystemComponent) :GameplayEffectClass "/Game/Game/Player/AbilitySystem/Effect/Add/GAS_GE_DrinkGourd.GAS_GE_DrinkGourd_C" :Level 1.0)))

(fn ConstructionScript
  (|BP->C++))

(fn CheckNearbyEnemiesbySphere
  (params (Radius :type Float%20%28double-precision%29))
  (bind _returnvalue (Transformation|GetActorLocation))
  (bind (_outhit _returnvalue_2) (Collision|SphereTraceForObjects _returnvalue (+ _returnvalue (* (Transformation|GetActorForwardVector) 1e+03)) Radius (Utilities|Array|MakeArray "ObjectTypeQuery7") false 0 "ForOneFrame"))
  (if _returnvalue_2
    (bind _asmokong_enemy (Utilities|Casting|CastToMokongEnemy (.HitActor (Collision|BreakHitResult _outhit))))
    (return _asmokong_enemy)))