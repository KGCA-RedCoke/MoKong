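; BP_Guangzhi is the player character Blueprint, wiring combat, camera lock-on and interaction input.
; It initializes CombatComponent with its mesh on BeginPlay, and primary action calls CheckCommit.
; Lock-on toggles the camera target to the nearest enemy or clears it, while interaction sends an Input.Interact gameplay event.
; The construction script hands Blueprint locomotion and parkour components to C++ references, and a forward sphere-trace helper finds MokongEnemy actors.
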(event EventBeginPlay
  (Class|CombatSystem|InitializeCombatSystem (Variables|Default|GetCombatComponent) (Variables|Character|GetMesh)))

(event Input|EnhancedActionEvents|EnhancedInputActionInputAction_Lockon
  (params (ActionValue :type Boolean) (ElapsedSeconds :type Float%20%28double-precision%29) (TriggeredSeconds :type Float%20%28double-precision%29) (InputAction :type Input%20Action%20Object%20Reference :default "/Game/Game/Data/Input/InputAction_Lockon.InputAction_Lockon"))
  (:Started
    (if (Class|MKPlayer|IsLockingon)
      (Utilities|HandleLockon 2.5e+03 :!label _label)
      (else
        (goto _label TryLockOn)))))

(event Input|EnhancedActionEvents|EnhancedInputActionInputAction_PrimaryAction
  (params (ActionValue :type Boolean) (ElapsedSeconds :type Float%20%28double-precision%29) (TriggeredSeconds :type Float%20%28double-precision%29) (InputAction :type Input%20Action%20Object%20Reference :default "/Game/Game/Data/Input/InputAction_PrimaryAction.InputAction_PrimaryAction"))
  (:Started
    (Class|CombatSystem|CheckCommit (Variables|Default|GetCombatComponent))))

(event Input|EnhancedActionEvents|EnhancedInputActionInputAction_Interaction
  (params (ActionValue :type Boolean) (ElapsedSeconds :type Float%20%28double-precision%29) (TriggeredSeconds :type Float%20%28double-precision%29) (InputAction :type Input%20Action%20Object%20Reference :default "/Game/Game/Data/Input/InputAction_Interaction.InputAction_Interaction"))
  (:Started
    (if (Variables|Default|GetbCanInteract)
      (Ability|SendGameplayEventtoActor self "(TagName=\"Input.Interact\")" (Variables|Default|GetInteractionPayload)))))

(fn ConstructionScript
  (|BP->C++))

(fn CheckNearbyEnemiesbySphere
  (params (Radius :type Float%20%28double-precision%29))
  (bind _returnvalue (Transformation|GetActorLocation))
  (bind (_outhit _returnvalue_2) (Collision|SphereTraceForObjects _returnvalue (+ _returnvalue (* (Transformation|GetActorForwardVector) 1e+03)) Radius (Utilities|Array|MakeArray "ObjectTypeQuery7") false 0 "ForOneFrame"))
  (if _returnvalue_2
    (bind _asmokong_enemy (Utilities|Casting|CastToMokongEnemy (.HitActor (Collision|BreakHitResult _outhit))))
    (return _asmokong_enemy)))