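; BP_TestUE5 is a test player Blueprint that links the base UE5 anim layer, sheathes the weapon on X and handles lock-on targeting.
; Lock-on input sphere-traces forward for a BP_Enemy_Guard and passes it to the camera's lock-on object.
; That object's target-change delegate toggles the enemy's lock-on widget, clearing the target when lost.
; A Blueprint-to-C++ graph assigns locomotion and parkour component references outside the CDO.
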(event Custom|OnTargetChangeDelegate_이벤트
  (params (NewTarget :type Actor%20Object%20Reference) (ChangeTargetReason :type EATPCChangeTargetReason%20Enum :default "SetNew"))
  (bind _target (Variables|Default|GetTarget)
    (:then
      (switch Utilities|FlowControl|Switch|SwitchonEATPCChangeTargetReason ChangeTargetReason
        (:SetNew
          (Class|MokongEnemy|ShowLockonWidget _target true))
        (:LostByExitCameraMode
          (Class|MokongEnemy|ShowLockonWidget _target false :!label _label)
          (Variables|Default|SetTarget 0))
        (:LostByDistance
          (goto _label))
        (:LostByVisible
          (goto _label))
        (:LostByPlayerInput
          (goto _label))))
    (:else)))

(event Custom|커스텀이벤트)

(event Input|EnhancedActionEvents|EnhancedInputActionInputAction_Lockon
  (params (ActionValue :type Boolean) (ElapsedSeconds :type Float%20%28double-precision%29) (TriggeredSeconds :type Float%20%28double-precision%29) (InputAction :type Input%20Action%20Object%20Reference :default "/Game/Game/Data/Input/InputAction_Lockon.InputAction_Lockon"))
  (bind _returnvalue (Transformation|GetActorLocation))
  (:Started
    (bind (_outhit _returnvalue_2) (Collision|SphereTraceForObjects _returnvalue (+ _returnvalue (* (Transformation|GetActorForwardVector) 1e+03)) 1e+03 (Utilities|Array|MakeArray "ObjectTypeQuery7") false 0 "ForOneFrame"))
    (if _returnvalue_2
      (bind _asbp_enemy_guard (Utilities|Casting|CastToBP_Enemy_Guard (.HitActor (Collision|BreakHitResult _outhit))))
      (Variables|Default|SetTarget _asbp_enemy_guard)
      (Class|ATPCCameraLockonTargetObject|SetTargetActor (Class|ATPCCameraComponent|GetCameraLockonTargetObject (Variables|Default|GetPlayerCam)) (.HitActor (Collision|BreakHitResult _outhit))))))

(event EventBeginPlay
  (Components|SkeletalMesh|AnimationBlueprintLinking|LinkAnimClassLayers (Variables|Character|GetMesh) "/Game/Game/Player/MovementSystem/Animation/Layer/ABP_UE5_Layer_Base.ABP_UE5_Layer_Base_C")
  (EventDispatchers|AssignOnTargetChangeDelegate (Class|ATPCCameraComponent|GetCameraLockonTargetObject (Variables|Default|GetPlayerCam)) (delegate Custom|OnTargetChangeDelegate_이벤트)))

(event Input|KeyboardEvents|X
  (params (Key :type Key%20Structure))
  (:Pressed
    (Class|WeaponBase|SheathWeapon (Variables|/Script/AbilitySystem.CombatSystem|GetCurrentWeapon (Variables|Default|GetCombatComponent)))))

(fn ConstructionScript
  (|BP->C++))