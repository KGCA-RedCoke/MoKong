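; Player locomotion Blueprint that routes Enhanced Input for movement, look, crouch and low profile to handler functions, and cycles movement models.
; An InputCondition macro uses a gate to classify secondary-action presses as started, held, released or tapped, forwarding only the held result.
; Helper functions cache the character's Ability System Component to apply sprint and jump stamina effects and remove sprint's.
; Jump, high-profile and overlay input handling is disconnected.
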(event EventBeginPlay)

(event EventTick
  (params (DeltaSeconds :type Float%20%28single-precision%29)))

(event Input|EnhancedActionEvents|EnhancedInputActionInputAction_Jump
  (params (ActionValue :type Boolean) (ElapsedSeconds :type Float%20%28double-precision%29) (TriggeredSeconds :type Float%20%28double-precision%29) (InputAction :type Input%20Action%20Object%20Reference :default "/Game/Game/Data/Input/InputAction_Jump.InputAction_Jump"))
  ;[0.1053 0.05995 0.1354] Jump Action Handler
)

(event Input|EnhancedActionEvents|EnhancedInputActionInputAction_HighProfile
  (params (ActionValue :type Boolean) (ElapsedSeconds :type Float%20%28double-precision%29) (TriggeredSeconds :type Float%20%28double-precision%29) (InputAction :type Input%20Action%20Object%20Reference :default "/Game/Game/Data/Input/InputAction_HighProfile.InputAction_HighProfile"))
  ;[0.1514 0.224 0.147] High Profile Action Handler
)

(event Input|EnhancedActionEvents|EnhancedInputActionInputAction_SecondaryAction
  (params (ActionValue :type Boolean) (ElapsedSeconds :type Float%20%28double-precision%29) (TriggeredSeconds :type Float%20%28double-precision%29) (InputAction :type Input%20Action%20Object%20Reference :default "/Game/Game/Data/Input/InputAction_SecondaryAction.InputAction_SecondaryAction"))
  ;[0.7344 0.4375 0.1415] Secondary Action (RMB) Handler
  (:Triggered
    (bind _inputresult (Utilities|InputCondition ElapsedSeconds 0.15 :!label _label))
    (Class|LocomotionComponent|HandleSecondaryProfileAction _inputresult ActionValue ElapsedSeconds))
  (:Started
    (goto _label Started))
  (:Completed
    (goto _label Completed)))

(event Input|EnhancedActionEvents|EnhancedInputActionInputAction_Movement
  (params (ActionValue :type Vector%202D%20Structure) (ElapsedSeconds :type Float%20%28double-precision%29) (TriggeredSeconds :type Float%20%28double-precision%29) (InputAction :type Input%20Action%20Object%20Reference :default "/Game/Game/Data/Input/InputAction_Movement.InputAction_Movement"))
  ;[0.07779 0.09786 0.2292] Movement And Look Input Handlers
  (:Triggered
    (Class|LocomotionComponent|HandleMovementInput ActionValue :!label _label))
  (:Completed
    (goto _label)))

(event Input|EnhancedActionEvents|EnhancedInputActionInputAction_Look
  (params (ActionValue :type Vector%202D%20Structure) (ElapsedSeconds :type Float%20%28double-precision%29) (TriggeredSeconds :type Float%20%28double-precision%29) (InputAction :type Input%20Action%20Object%20Reference :default "/Game/Game/Data/Input/InputAction_Look.InputAction_Look"))
  ;[0.07779 0.09786 0.2292] Movement And Look Input Handlers
  (:Triggered
    (Class|LocomotionComponent|HandleLookInput ActionValue :!label _label))
  (:Completed
    (goto _label)))

(event Input|EnhancedActionEvents|EnhancedInputActionInputAction_LowProfile
  (params (ActionValue :type Boolean) (ElapsedSeconds :type Float%20%28double-precision%29) (TriggeredSeconds :type Float%20%28double-precision%29) (InputAction :type Input%20Action%20Object%20Reference :default "/Game/Game/Data/Input/InputAction_LowProfile.InputAction_LowProfile"))
  ;[0.1514 0.224 0.147] Low Profile Action Handler
  (:Triggered
    (Class|LocomotionComponent|HandleLowProfileAction ActionValue ElapsedSeconds :!label _label))
  (:Canceled
    (goto _label)))

(event Input|EnhancedActionEvents|EnhancedInputActionInputAction_Crouch
  (params (ActionValue :type Boolean) (ElapsedSeconds :type Float%20%28double-precision%29) (TriggeredSeconds :type Float%20%28double-precision%29) (InputAction :type Input%20Action%20Object%20Reference :default "/Game/Game/Data/Input/InputAction_Crouch.InputAction_Crouch"))
  ;[0.1053 0.05995 0.1354] Crouch Action Handler
  (Class|LocomotionComponent|HandleCrouchAction ActionValue ElapsedSeconds))

(event Input|EnhancedActionEvents|EnhancedInputActionInputAction_ToggleMovementModel
  (params (ActionValue :type Boolean) (ElapsedSeconds :type Float%20%28double-precision%29) (TriggeredSeconds :type Float%20%28double-precision%29) (InputAction :type Input%20Action%20Object%20Reference :default "/Game/Game/Data/Input/InputAction_ToggleMovementModel.InputAction_ToggleMovementModel"))
  ;[0.07779 0.09786 0.2292] Toggle Movement Model
  (Class|LocomotionComponent|SetMovementModel (Utilities|Select :Index (Variables|Default|GetCurrentMovementModel) :None "Normal" :Normal "Sluggish" :Sluggish "Responsive" :Responsive "Normal")))

(event Input|EnhancedActionEvents|EnhancedInputActionInputAction_OverlayMenu
  (params (ActionValue :type Boolean) (ElapsedSeconds :type Float%20%28double-precision%29) (TriggeredSeconds :type Float%20%28double-precision%29) (InputAction :type Input%20Action%20Object%20Reference :default "/Game/Game/Data/Input/InputAction_OverlayMenu.InputAction_OverlayMenu")))

(event Input|EnhancedActionEvents|EnhancedInputActionInputAction_Movement
  (params (ActionValue :type Vector%202D%20Structure) (ElapsedSeconds :type Float%20%28double-precision%29) (TriggeredSeconds :type Float%20%28double-precision%29) (InputAction :type Input%20Action%20Object%20Reference :default "/Game/Game/Data/Input/InputAction_Movement.InputAction_Movement"))
  ;[0.07779 0.09786 0.2292] Movement And Look Input Handlers
  (:Triggered
    (Class|LocomotionComponentBase|HandleInput ActionValue :!label _label))
  (:Canceled
    (goto _label))
  (:Completed
    (goto _label)))

(fn ApplySprintEffect
  (if (Utilities|Enum|Equal(Enum) (Variables|Default|GetDesiredGaitProfile) "High")
    (CallFunction|CheckASC)
    (GameplayEffects|ApplyGameplayEffectToSelf :self (Variables|Default|GetAbilitySystemComponent) :GameplayEffectClass "/Game/Game/Player/AbilitySystem/Effect/Cost/GAS_Cost_Stamina_Sprint.GAS_Cost_Stamina_Sprint_C")))

(fn ApplyJumpEffect
  (CallFunction|CheckASC)
  (GameplayEffects|ApplyGameplayEffectToSelf :self (Variables|Default|GetAbilitySystemComponent) :GameplayEffectClass "/Game/Game/Player/AbilitySystem/Effect/Cost/GAS_Cost_Stamina_Jump.GAS_Cost_Stamina_Jump_C"))

(fn RemoveSprintEffect
  (if (Utilities|Enum|Equal(Enum) (Variables|Default|GetDesiredGaitProfile) "Mid")
    (CallFunction|CheckASC)
    (GameplayEffects|RemoveActiveGameplayEffect :self (Variables|Default|GetAbilitySystemComponent))))

(fn CheckASC
  (Variables|Default|GetAbilitySystemComponent
    (:then
      _)
    (:else
      (Variables|Default|SetAbilitySystemComponent (Ability|GetAbilitySystemComponent (Class|LocomotionComponentBase|GetCharacter)))))
  (return))