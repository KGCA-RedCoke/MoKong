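; Short-lived Wukong replica actor that displays a set of equipment meshes and removes itself after ten seconds.
; The construction script copies mesh variables onto separate shoes, suit, gloves and helmet skeletal mesh components.
; BeginPlay only sets the lifespan; the overlap and tick events are empty.
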(event EventBeginPlay
  (Actor|SetLifeSpan 1e+01))

(event Collision|EventActorBeginOverlap
  (params (OtherActor :type Actor%20Object%20Reference)))

(event EventTick
  (params (DeltaSeconds :type Float%20%28single-precision%29)))

(fn ConstructionScript
  (Variables|/Script/Engine.SkeletalMeshComponent|SetSkeletalMeshAsset (Variables|Default|GetShoes) (Variables|Default|GetFeetMesh))
  (Variables|/Script/Engine.SkeletalMeshComponent|SetSkeletalMeshAsset (Variables|Default|GetSuit) (Variables|Default|GetSuitMesh))
  (Variables|/Script/Engine.SkeletalMeshComponent|SetSkeletalMeshAsset (Variables|Default|GetGloves) (Variables|Default|GetGlovesMesh))
  (Variables|/Script/Engine.SkeletalMeshComponent|SetSkeletalMeshAsset (Variables|Default|GetHelmet) (Variables|Default|GetHelmetMesh)))