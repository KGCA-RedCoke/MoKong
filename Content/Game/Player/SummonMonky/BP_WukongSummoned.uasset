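; BP_WukongSummoned is a summoned Wukong clone character with a limited lifespan that can perform a primary attack.
; On BeginPlay it sets up high-profile locomotion and the combat component, plays a summon montage, then times a disappear montage to just before its lifespan ends.
; Attack runs a combat commit check and activates the primary-attack gameplay ability.
; The construction script builds the modular armor meshes, slaved to the main mesh via leader pose.
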(event Custom|커스텀이벤트
  (Animation|PlayAnimMontage "/Game/Game/Player/Animation/Montages/MTG_WK_Disappear.MTG_WK_Disappear" 1.0 "None"))

(event EventBeginPlay
  (Class|LocomotionComponent|HandleHighProfileAction (Variables|Default|GetBP_Locomotion) true 0.0)
  (Class|CombatSystem|InitializeCombatSystem (Variables|Default|GetCombatComponent) (Variables|Character|GetMesh))
  (Utilities|FlowControl|Delay 0.05)
  (Animation|PlayAnimMontage "/Game/Game/Player/Animation/Montages/MTG_WK_Summoned.MTG_WK_Summoned" 1.0 "None")
  (Utilities|Time|SetTimerbyEvent (delegate Custom|커스텀이벤트) (- (Actor|GetLifeSpan) 0.8) false true))

(event Collision|EventActorBeginOverlap
  (params (OtherActor :type Actor%20Object%20Reference)))

(event EventTick
  (params (DeltaSeconds :type Float%20%28single-precision%29)))

(event EventAttack
  (params (AbilityClass :type MK%20Gameplay%20Ability%20Class%20Reference) (AttackType :type Byte :default 0))
  (Class|CombatSystem|CheckCommit (Variables|Default|GetCombatComponent))
  (Abilities|TryActivateAbilitybyClass (Variables|Default|GetAbilitySystemComponent) "/Game/Game/Player/AbilitySystem/Ability/GAS_GA_PrimaryAttack.GAS_GA_PrimaryAttack_C" true))

(event EventDestroyed)

(fn ConstructionScript
  (Variables|/Script/Engine.SkeletalMeshComponent|SetSkeletalMeshAsset (Variables|Default|GetShoes) (Variables|Default|GetFeetMesh))
  (Variables|/Script/Engine.SkeletalMeshComponent|SetSkeletalMeshAsset (Variables|Default|GetSuit) (Variables|트랜스포메이션|GetSuitMesh))
  (Variables|/Script/Engine.SkeletalMeshComponent|SetSkeletalMeshAsset (Variables|Default|GetGloves) (Variables|Default|GetGlovesMesh))
  (Variables|/Script/Engine.SkeletalMeshComponent|SetSkeletalMeshAsset (Variables|Default|GetHelmet) (Variables|Default|GetHelmetMesh))
  (Components|SkinnedMesh|SetLeaderPoseComponent (Variables|Default|GetGloves) (Variables|Character|GetMesh) false false))

(fn GetPatrolRoute
  (return 0))