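; BP_WukongAIController is the AI controller for the player's summoned Wukong (monkey) pawn.
; On BeginPlay it runs BT_WukongSummoned and stores the instigator as PlayerRef and the pawn's ability system component as OwnerASC in the blackboard.
; Perception updates ignore the player character and are classified by sense.
; Sight triggers HandleSenseSight and writes the KeyTarget blackboard key, while hearing is classified but left unhandled.
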(event OnTargetPerceptionUpdated(PerceptionComponent)
  (params (Actor :type Actor%20Object%20Reference) (Stimulus :type AI%20Stimulus%20Structure))
  (if (!= Actor (Game|GetPlayerCharacter 0))
    (Utilities|ClssifyStimulus Stimulus
      (:Sight
        (Class|CrowdEnemyAIController|HandleSenseSight Actor)
        (AI|Components|Blackboard|SetValueasObject (AI|GetBlackboard 0) (Variables|Default|GetKey_Target) 0)))))

(event EventBeginPlay
  (bind _returnvalue (AI|GetBlackboard 0))
  (AI|RunBehaviorTree "/Game/Game/Player/Tree/BT_WukongSummoned.BT_WukongSummoned")
  (AI|Components|Blackboard|SetValueasObject _returnvalue (Utilities|Name|MakeLiteralName "PlayerRef") (Game|GetInstigator))
  (AI|Components|Blackboard|SetValueasObject _returnvalue (Utilities|Name|MakeLiteralName "OwnerASC") (Ability|GetAbilitySystemComponent (Pawn|GetControlledPawn))))

(fn ConstructionScript)