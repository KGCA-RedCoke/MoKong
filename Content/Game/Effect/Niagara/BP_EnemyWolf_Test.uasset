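; BP_EnemyWolf_Test is a test enemy wolf Blueprint that tries a temporary material swap for a vaporization skill.
; On BeginPlay it caches the mesh materials, applies TransparentMaterial to every slot, then restores the originals after a fixed delay.
; TransparentMaterial is set to None first, so the swap assigns no material.
; Combo attack and hearing events are empty, and player-sighting calls the parent.
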(event EventBeginPlay
  (|CallParentFunction)
  ;[0.01096 0.01161 0.0137] 기화술 머티리얼 바꾸기
  (Variables|Default|SetTransparentMaterial 0)
  (for _array_element (Rendering|Material|GetMaterials (Variables|Character|GetMesh))
    (Utilities|Array|Add (Variables|Default|GetOriginalMaterials) _array_element))
  (for _index (range 0 (- (Rendering|Material|GetNumMaterials (Variables|Character|GetMesh)) 1))
    (Rendering|Material|SetMaterial (Variables|Character|GetMesh) _index (Variables|Default|GetTransparentMaterial)))
  (Utilities|FlowControl|Delay 5.0)
  (for (_array_element_2 _array_index) (Variables|Default|GetOriginalMaterials)
    (Rendering|Material|SetMaterial (Variables|Character|GetMesh) _array_index _array_element_2)))

(event Collision|EventActorBeginOverlap
  (params (OtherActor :type Actor%20Object%20Reference))
  (|CallParentFunction OtherActor) ; 지금 이 노드는 비활성 상태입니다. \n핀을 끌어서 다른 노드를 연결하면 활성화됩니다.
)

(event EventTick
  (params (DeltaSeconds :type Float%20%28single-precision%29))
  (|CallParentFunction DeltaSeconds) ; 지금 이 노드는 비활성 상태입니다. \n핀을 끌어서 다른 노드를 연결하면 활성화됩니다.
)

(event EventTryComboAttack)

(event EventOnHeardSomething
  (params (Location :type Vector%20%28by%20ref%29 :default "0, 0, 0")))

(event EventOnPlayerSeen
  (params (Target :type Actor%20Object%20Reference))
  (|CallParentFunction Target))

(fn ConstructionScript
  (|CallParentFunction))