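; Base interactable prop that shows an interaction prompt and registers itself with the Wukong player character.
; On BeginPlay it caches the player and prompt widget, whose visibility follows an outer sphere's overlaps.
; An inner sphere switches the widget image, toggles the player's CanInteract and puts itself in or clears the player's InteractionPayload.
; Overlapping OpenPoint sends an OpenBox gameplay event to that actor, then disables OpenPoint's collision.
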(event EventBeginPlay
  (|SetReference))

(event Collision|EventActorBeginOverlap
  (params (OtherActor :type Actor%20Object%20Reference)))

(event EventTick
  (params (DeltaSeconds :type Float%20%28single-precision%29)))

(event OnComponentBeginOverlap(InnerInteractionSphere)
  (params (OverlappedComponent :type Primitive%20Component%20Object%20Reference) (OtherActor :type Actor%20Object%20Reference) (OtherComp :type Primitive%20Component%20Object%20Reference) (OtherBodyIndex :type Integer) (bFromSweep :type Boolean) (SweepResult :type Hit%20Result%20Structure%20%28by%20ref%29))
  (CallFunction|SetInteraction true))

(event OnComponentBeginOverlap(OuterInteractionSphere)
  (params (OverlappedComponent :type Primitive%20Component%20Object%20Reference) (OtherActor :type Actor%20Object%20Reference) (OtherComp :type Primitive%20Component%20Object%20Reference) (OtherBodyIndex :type Integer) (bFromSweep :type Boolean) (SweepResult :type Hit%20Result%20Structure%20%28by%20ref%29))
  (Rendering|SetVisibility (Variables|Default|GetInteractionWidgetComponent) true false))

(event OnComponentEndOverlap(OuterInteractionSphere)
  (params (OverlappedComponent :type Primitive%20Component%20Object%20Reference) (OtherActor :type Actor%20Object%20Reference) (OtherComp :type Primitive%20Component%20Object%20Reference) (OtherBodyIndex :type Integer))
  (Rendering|SetVisibility (Variables|Default|GetInteractionWidgetComponent) false false))

(event OnComponentEndOverlap(InnerInteractionSphere)
  (params (OverlappedComponent :type Primitive%20Component%20Object%20Reference) (OtherActor :type Actor%20Object%20Reference) (OtherComp :type Primitive%20Component%20Object%20Reference) (OtherBodyIndex :type Integer))
  (CallFunction|SetInteraction false))

(event OnComponentBeginOverlap(OpenPoint)
  (params (OverlappedComponent :type Primitive%20Component%20Object%20Reference) (OtherActor :type Actor%20Object%20Reference) (OtherComp :type Primitive%20Component%20Object%20Reference) (OtherBodyIndex :type Integer) (bFromSweep :type Boolean) (SweepResult :type Hit%20Result%20Structure%20%28by%20ref%29))
  (Ability|SendGameplayEventtoActor OtherActor "(TagName=\"Event.Wukong.OpenBox\")")
  (Collision|SetCollisionEnabled (Variables|Default|GetOpenPoint) "NoCollision"))

(fn ConstructionScript)

(fn SetInteraction
  (params (bCanInteract :type Boolean))
  (bind _playerref (Variables|Default|GetPlayerRef))
  (Default|SwitchImage (Variables|Default|GetWidgetRef) bCanInteract)
  (Variables|/Script/MoKong.MKPlayer|SetbCanInteract _playerref bCanInteract)
  (Variables|/Game/Game/Player/BP_Wukong.BP_Wukong_C|SetInteractionPayload _playerref (Utilities|Struct|MakeGameplayEventData "(TagName=\"\")" 0 0 (Utilities|SelectObject self 0 bCanInteract) 0 "()" "(GameplayTags=)" "(GameplayTags=)" 0.0 "()")))